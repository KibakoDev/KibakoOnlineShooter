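; Parent Blueprint for first-person weapons that provides the firing effects.
; BeginPlay caches its owner as the PlayerCharacter_BP reference.
; FireWeapon, if that reference is valid, attaches a pistol muzzle flash at the muzzle location and plays layered one-shot, stop and tail pistol sounds in 2D.
; It contains no projectile, trace or damage logic.
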(event Custom|FireWeapon
  (Utilities|IsValid (Variables|References|GetAs%20Player%20Character%20BP)
    (:Is%20Valid
      (Effects|SpawnEmitterAttached "/Game/FX/MilitaryWeapDark/FX/P_Pistol_MuzzleFlash_01.P_Pistol_MuzzleFlash_01" (Variables|Default|GetWeaponMuzzleLoc) "None" "0, 0, 0" "0, 0, 0" "0.500000,0.500000,0.500000" "SnapToTarget")
      (Audio|PlaySound2D "/Weapons_Sounds_III/Audio/Cues/3_07_PISTOL/3_07_PISTOL_Oneshot_Cue.3_07_PISTOL_Oneshot_Cue" 1.0 1.0 0.0 0 0)
      (Audio|PlaySound2D "/Weapons_Sounds_III/Audio/Cues/3_07_PISTOL/3_07_PISTOL_Stop_cue.3_07_PISTOL_Stop_cue" 1.0 1.0 0.0 0 0)
      (Audio|PlaySound2D "/Weapons_Sounds_III/Audio/Cues/3_07_PISTOL/3_07_PISTOL_Tail_Cue.3_07_PISTOL_Tail_Cue" 1.0 1.0 0.0 0 0))))

(event EventBeginPlay
  (bind _asplayer_character_bp (Utilities|Casting|CastToPlayerCharacter_BP (Components|GetOwner)))
  (Variables|References|SetAs%20Player%20Character%20BP _asplayer_character_bp))

(fn ConstructionScript)